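; BP_TutoPawn is a pawn, apparently for a tutorial, that drives a panel cursor (PaneruS) over a grid to swap tiles.
; Directional inputs step the cursor, and ActionSelect alternates between marking and swapping BP_Block or BP_Paneru actors, found by matching XY location.
; Needle and arrow swap branches exist, but nothing here selects those types.
; ActionPrincessChange checks tagged princess actors' death and hit flags, then toggles UserPrincessNow through a delay timeline.
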(event `self.ReceiveBeginPlay`
  (set `self.location` (`SceneComponent.K2_GetComponentLocation` (`self.paneru_s`))))

(event `InputAction|ActionUp`
  (params (Key :type "Key Structure"))
  (:`Pressed`
    (bind _output_get (set `self.location` (+ (`self.location`) (-220.0 0.0 0.0))))
    (`SceneComponent.K2_SetWorldLocation` (`self.paneru_s`) _output_get false false)))

(event `InputAction|ActionDown`
  (params (Key :type "Key Structure"))
  (:`Pressed`
    (bind _output_get (set `self.location` (+ (`self.location`) (220.0 0.0 0.0))))
    (`SceneComponent.K2_SetWorldLocation` (`self.paneru_s`) _output_get false false)))

(event `InputAction|ActionRight`
  (params (Key :type "Key Structure"))
  (:`Pressed`
    (bind _output_get (set `self.location` (+ (`self.location`) (0.0 -200.0 0.0))))
    (`SceneComponent.K2_SetWorldLocation` (`self.paneru_s`) _output_get false false)))

(event `InputAction|ActionLeft`
  (params (Key :type "Key Structure"))
  (:`Pressed`
    (bind _output_get (set `self.location` (+ (`self.location`) (0.0 200.0 0.0))))
    (`SceneComponent.K2_SetWorldLocation` (`self.paneru_s`) _output_get false false)))

(event `InputAction|ActionPrincessChange`
  (params (Key :type "Key Structure"))
  (:`Pressed`
    (bind _outactors (`GameplayStatics.GetAllActorsOfClass` "/Game/My/BP/BP_Princess.BP_Princess_C"))
    (for _array_element _outactors
      (if (`self.ActorHasTag` _array_element "MainCharacter_P")
        (if (not (`/Game/My/BP/BP_Princess.DeathNow` _array_element))
          (bind _outactors_2 (`GameplayStatics.GetAllActorsOfClass` "/Game/My/BP/BP_ChangePrincess.BP_ChangePrincess_C"))
          (for _array_element_2 _outactors_2
            (if (`self.ActorHasTag` _array_element_2 "MainCharacter_CP")
              (if (`/Game/My/BP/BP_ChangePrincess.BlockHit` _array_element_2)
                _
                (elif (`/Game/My/BP/BP_ChangePrincess.DevilHit` _array_element_2)
                  _
                  (elif (== (`self.TimeLineTime`) 1.0)
                    (bind (_direction `_新規track_0`) (`Timeline|ChangeDelayTimeLine` :!via `PlayFromStart`)
                      (:`Update`
                        (set `self.TimeLineTime` `_新規track_0`)
                        (if (<= `_新規track_0` 0.0)
                          (set `self.UserPrincessNow` (not (`self.UserPrincessNow`))))))))))))))))

(event `self.ReceiveTick`
  (params (DeltaSeconds :type "Float (single-precision)")))

(event `InputAction|ActionSelect`
  (params (Key :type "Key Structure"))
  (bind (_location_x _location_y) (`KismetMathLibrary.BreakVector` (`self.location`)))
  (bind (_location_x_2 _location_y_2) (`KismetMathLibrary.BreakVector` (`self.location`)))
  (bind _bp_block (`self.BP_Block`))
  (bind (_location_x_3 _location_y_3) (`KismetMathLibrary.BreakVector` (`self.location`)))
  (bind (_location_x_4 _location_y_4) (`KismetMathLibrary.BreakVector` (`self.location`)))
  (bind _bp_needle (`self.BP_Needle`))
  (bind _bp_paneru (`self.BP_Paneru`))
  (bind _bp_arrow (`self.BP_Arrow`))
  (bind _bp_block_2 (`self.BP_Block`))
  (bind _bp_needle_2 (`self.BP_Needle`))
  (bind _bp_paneru_2 (`self.BP_Paneru`))
  (bind _bp_arrow_2 (`self.BP_Arrow`))
  (:`Pressed`
    (bind _output_get (set `self.ClickCheck` (not (`self.ClickCheck`))))
    (if _output_get
      ;[1 1 1] どれかのBP_Blockの判定
      (bind _outactors (`GameplayStatics.GetAllActorsOfClass` "/Game/My/BP/BP_Block.BP_Block_C"))
      (for _array_element _outactors
        (bind (_location_x_5 _location_y_5) (`KismetMathLibrary.BreakVector` (`/Game/My/BP/BP_Block.Location` _array_element)))
        (if (== (`KismetMathLibrary.MakeVector` _location_x_5 _location_y_5) (`KismetMathLibrary.MakeVector` _location_x_3 _location_y_3))
          (set `/Game/My/BP/BP_Block.ClickCheck` true _array_element)
          (set `self.BP_Block` _array_element)
          (set `self.BlockClick` true)
          ;[1 1 1] どれかのBP_Paneruか判定
          (bind _outactors_2 (`GameplayStatics.GetAllActorsOfClass` "/Game/My/BP/BP_Paneru.BP_Paneru_C"))
          (for _array_element_2 _outactors_2
            (bind (_location_x_6 _location_y_6) (`KismetMathLibrary.BreakVector` (`/Game/My/BP/BP_Paneru.Location` _array_element_2)))
            (if (== (`KismetMathLibrary.MakeVector` _location_x_6 _location_y_6) (`KismetMathLibrary.MakeVector` _location_x_4 _location_y_4))
              (set `/Game/My/BP/BP_Paneru.ClickCheck` true _array_element_2)
              (set `self.BP_Paneru` _array_element_2)
              (set `self.PaneruClick` true)))))
      (else
        ;[1 1 1] 相手がブロックの時
        (bind _outactors_3 (`GameplayStatics.GetAllActorsOfClass` "/Game/My/BP/BP_Block.BP_Block_C"))
        (for _array_element_3 _outactors_3
          (bind (_location_x_7 _location_y_7) (`KismetMathLibrary.BreakVector` (`/Game/My/BP/BP_Block.Location` _array_element_3)))
          (if (== (`KismetMathLibrary.MakeVector` _location_x_7 _location_y_7) (`KismetMathLibrary.MakeVector` _location_x _location_y))
            (set `self.BP_BlockCheck` _array_element_3)
            (set `self.tempLocation` (`/Game/My/BP/BP_Block.Location` _array_element_3))
            (if (`self.BlockClick`)
              (`self.K2_SetActorLocation` (`self.BP_BlockCheck`) (`/Game/My/BP/BP_Block.Location` (`self.BP_Block`)) false false)
              (set `/Game/My/BP/BP_Block.Location` (`/Game/My/BP/BP_Block.Location` (`self.BP_Block`)) (`self.BP_BlockCheck`))
              (`self.K2_SetActorLocation` (`self.BP_Block`) (`self.tempLocation`) false false)
              (set `/Game/My/BP/BP_Block.Location` (`self.tempLocation`) _bp_block)
              (set `/Game/My/BP/BP_Block.ClickCheck` false _bp_block)
              (set `self.BlockClick` false)
              (elif (`self.NeedleClick`)
                (`self.K2_SetActorLocation` (`self.BP_BlockCheck`) (`/Game/My/BP/BP_Needle.Location` (`self.BP_Needle`)) false false)
                (set `/Game/My/BP/BP_Block.Location` (`/Game/My/BP/BP_Needle.Location` (`self.BP_Needle`)) (`self.BP_BlockCheck`))
                (`self.K2_SetActorLocation` (`self.BP_Needle`) (`self.tempLocation`) false false)
                (set `/Game/My/BP/BP_Needle.Location` (`self.tempLocation`) _bp_needle)
                (set `/Game/My/BP/BP_Needle.ClickCheck` false _bp_needle)
                (set `self.NeedleClick` false)
                (elif (`self.PaneruClick`)
                  (`self.K2_SetActorLocation` (`self.BP_BlockCheck`) (`/Game/My/BP/BP_Paneru.Location` (`self.BP_Paneru`)) false false)
                  (set `/Game/My/BP/BP_Block.Location` (`/Game/My/BP/BP_Paneru.Location` (`self.BP_Paneru`)) (`self.BP_BlockCheck`))
                  (`self.K2_SetActorLocation` (`self.BP_Paneru`) (`self.tempLocation`) false false)
                  (set `/Game/My/BP/BP_Paneru.Location` (`self.tempLocation`) _bp_paneru)
                  (set `/Game/My/BP/BP_Paneru.ClickCheck` false _bp_paneru)
                  (set `self.PaneruClick` false)
                  (else
                    ;;[1 1 1] なくてもいいかも
                    (if (`self.ArrowClick`)
                      (`self.K2_SetActorLocation` (`self.BP_BlockCheck`) (`/Game/My/BP/BP_Arrow.Location` (`self.BP_Arrow`)) false false)
                      (set `/Game/My/BP/BP_Block.Location` (`/Game/My/BP/BP_Arrow.Location` (`self.BP_Arrow`)) (`self.BP_BlockCheck`))
                      (`self.K2_SetActorLocation` (`self.BP_Arrow`) (`self.tempLocation`) false false)
                      (set `/Game/My/BP/BP_Arrow.Location` (`self.tempLocation`) _bp_arrow)
                      (set `/Game/My/BP/BP_Arrow.ClickCheck` false _bp_arrow)
                      (set `self.ArrowClick` false))))))
            (else
              ;[1 1 1] 相手がパネルの時
              (bind _outactors_4 (`GameplayStatics.GetAllActorsOfClass` "/Game/My/BP/BP_Paneru.BP_Paneru_C"))
              (for _array_element_4 _outactors_4
                (bind (_location_x_8 _location_y_8) (`KismetMathLibrary.BreakVector` (`/Game/My/BP/BP_Paneru.Location` _array_element_4)))
                (if (== (`KismetMathLibrary.MakeVector` _location_x_8 _location_y_8) (`KismetMathLibrary.MakeVector` _location_x_2 _location_y_2))
                  (set `self.BP_PaneruCheck` _array_element_4)
                  (set `self.tempLocation` (`/Game/My/BP/BP_Paneru.Location` _array_element_4))
                  (if (`self.BlockClick`)
                    (`self.K2_SetActorLocation` (`self.BP_PaneruCheck`) (`/Game/My/BP/BP_Block.Location` (`self.BP_Block`)) false false)
                    (set `/Game/My/BP/BP_Paneru.Location` (`/Game/My/BP/BP_Block.Location` (`self.BP_Block`)) (`self.BP_PaneruCheck`))
                    (`self.K2_SetActorLocation` (`self.BP_Block`) (`self.tempLocation`) false false)
                    (set `/Game/My/BP/BP_Block.Location` (`self.tempLocation`) _bp_block_2)
                    (set `/Game/My/BP/BP_Block.ClickCheck` false _bp_block_2)
                    (set `self.BlockClick` false)
                    (elif (`self.NeedleClick`)
                      (`self.K2_SetActorLocation` (`self.BP_PaneruCheck`) (`/Game/My/BP/BP_Needle.Location` (`self.BP_Needle`)) false false)
                      (set `/Game/My/BP/BP_Paneru.Location` (`/Game/My/BP/BP_Needle.Location` (`self.BP_Needle`)) (`self.BP_PaneruCheck`))
                      (`self.K2_SetActorLocation` (`self.BP_Needle`) (`self.tempLocation`) false false)
                      (set `/Game/My/BP/BP_Needle.Location` (`self.tempLocation`) _bp_needle_2)
                      (set `/Game/My/BP/BP_Needle.ClickCheck` false _bp_needle_2)
                      (set `self.NeedleClick` false)
                      (elif (`self.PaneruClick`)
                        (`self.K2_SetActorLocation` (`self.BP_PaneruCheck`) (`/Game/My/BP/BP_Paneru.Location` (`self.BP_Paneru`)) false false)
                        (set `/Game/My/BP/BP_Paneru.Location` (`/Game/My/BP/BP_Paneru.Location` (`self.BP_Paneru`)) (`self.BP_PaneruCheck`))
                        (`self.K2_SetActorLocation` (`self.BP_Paneru`) (`self.tempLocation`) false false)
                        (set `/Game/My/BP/BP_Paneru.Location` (`self.tempLocation`) _bp_paneru_2)
                        (set `/Game/My/BP/BP_Paneru.ClickCheck` false _bp_paneru_2)
                        (set `self.PaneruClick` false)
                        (else
                          ;;[1 1 1] なくてもいいかも
                          (if (`self.ArrowClick`)
                            (`self.K2_SetActorLocation` (`self.BP_PaneruCheck`) (`/Game/My/BP/BP_Arrow.Location` (`self.BP_Arrow`)) false false)
                            (set `/Game/My/BP/BP_Paneru.Location` (`/Game/My/BP/BP_Arrow.Location` (`self.BP_Arrow`)) (`self.BP_PaneruCheck`))
                            (`self.K2_SetActorLocation` (`self.BP_Arrow`) (`self.tempLocation`) false false)
                            (set `/Game/My/BP/BP_Arrow.Location` (`self.tempLocation`) _bp_arrow_2)
                            (set `/Game/My/BP/BP_Arrow.ClickCheck` false _bp_arrow_2)
                            (set `self.ArrowClick` false)))))))))))))))

(fn `UserConstructionScript`)