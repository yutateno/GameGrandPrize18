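; Golem character that walks along its forward Y direction once the player pawn's AnyButtonCheck is set.
; Capsule hits check tags on all actors of the hit class, setting flags for blocks, princess, changed princess and needles.
; Tick reads these flags to pause movement or trigger death, which also occurs near a BP_BackBoss on Y.
; Death disables mesh and capsule collision, then destroys the actor after a delay.
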(event `self.ReceiveBeginPlay`
  ;[1 1 1] 初期化
  (set `self.DeathNow` false)
  (set `self.BlockHit` false)
  (set `self.PrincessHit` false)
  (set `self.ChangePrincessHit` false))

(event `self.ReceiveTick`
  (params (DeltaSeconds :type "Float (single-precision)"))
  (bind (_returnvalue_x _returnvalue_y) (`KismetMathLibrary.BreakVector` (`self.GetActorForwardVector`)))
  (bind (_returnvalue_x_2 _returnvalue_y_2) (`KismetMathLibrary.BreakVector` (`self.K2_GetActorLocation`)))
  (bind _asbp_test_pawn (cast `/Game/My/BP/BP_TestPawn` (`GameplayStatics.GetPlayerPawn` 0)))
  (if (`/Game/My/BP/BP_TestPawn.AnyButtonCheck` _asbp_test_pawn)
    (bind _outactors (`GameplayStatics.GetAllActorsOfClass` "/Game/My/BP/BP_BackBoss.BP_BackBoss_C"))
    (for _array_element _outactors
      (bind (_location_x _location_y) (`KismetMathLibrary.BreakVector` (`/Game/My/BP/BP_BackBoss.location` _array_element)))
      (if (== (`KismetMathLibrary.MakeVector` 0.0 _location_y) (`KismetMathLibrary.MakeVector` 0.0 _returnvalue_y_2) :`ErrorTolerance` 300.0)
        (set `self.DeathNow` true)
        (`/Engine/EditorBlueprintResources/StandardMacros.DoOnce` false :!label _label
          (:`Completed`
            (`PrimitiveComponent.SetCollisionEnabled` (`self.Mesh`) "NoCollision")
            (`PrimitiveComponent.SetCollisionEnabled` (`self.CapsuleComponent`) "NoCollision")
            (`KismetSystemLibrary.Delay` 1.52)
            (`self.K2_DestroyActor`)))
        (elif (`self.DeathNow`)
          (goto _label)
          (elif (`self.BlockHit`)
            (`KismetSystemLibrary.Delay` 0.4)
            (set `self.BlockHit` false)
            (else
              (if (`self.PrincessHit`)
                (`KismetSystemLibrary.Delay` 1.0)
                (set `self.PrincessHit` false))
              (if (`self.ChangePrincessHit`)
                (`KismetSystemLibrary.Delay` 4.4)
                (set `self.DeathNow` true)
                (goto _label)
                (else
                  (`self.AddMovementInput` (`KismetMathLibrary.MakeVector` 0.0 _returnvalue_y)))))))))))

(event `self.CapsuleComponent.OnComponentHit`
  (params (HitComponent :type "PrimitiveComponent Object Reference") (OtherActor :type "Actor Object Reference") (OtherComp :type "PrimitiveComponent Object Reference") (NormalImpulse :type "Vector Structure") (Hit :type "HitResult Structure (by ref)"))
  (`self.BlockHitFunc` OtherActor)
  (`self.PrincessHitFunc` OtherActor)
  (`self.ChangePrincessHitFunc` OtherActor)
  (`self.NeedleHitFunc` OtherActor))

(fn `BlockHitFunc`
  (params (`Other Pawn` :type "Actor Object Reference"))
  (bind _outactors (`GameplayStatics.GetAllActorsOfClass` (`GameplayStatics.GetObjectClass` `Other Pawn`)))
  (for _array_element _outactors
    (set `self.BlockHit` (`self.ActorHasTag` _array_element "Block"))))

(fn `ChangePrincessHitFunc`
  (params (`Other Pawn` :type "Actor Object Reference"))
  (bind _outactors (`GameplayStatics.GetAllActorsOfClass` (`GameplayStatics.GetObjectClass` `Other Pawn`)))
  (for _array_element _outactors
    (if (`self.ActorHasTag` _array_element "MainCharacter_CP")
      (`/Engine/EditorBlueprintResources/StandardMacros.DoOnce` false
        (:`Completed`
          (set `self.ChangePrincessHit` true))))))

(fn `NeedleHitFunc`
  (params (`Other Pawn` :type "Actor Object Reference"))
  (bind _outactors (`GameplayStatics.GetAllActorsOfClass` (`GameplayStatics.GetObjectClass` `Other Pawn`)))
  (for _array_element _outactors
    (set `self.DeathNow` (`self.ActorHasTag` _array_element "Needle"))))

(fn `PrincessHitFunc`
  (params (`Other Pawn` :type "Actor Object Reference"))
  (bind _outactors (`GameplayStatics.GetAllActorsOfClass` (`GameplayStatics.GetObjectClass` `Other Pawn`)))
  (for _array_element _outactors
    (if (`self.ActorHasTag` _array_element "MainCharacter_P")
      (`/Engine/EditorBlueprintResources/StandardMacros.DoOnce` false
        (:`Completed`
          (set `self.PrincessHit` true))))))

(fn `UserConstructionScript`)