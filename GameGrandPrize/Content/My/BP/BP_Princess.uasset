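; Princess character that auto-runs along Y and swaps in and out of play as BP_TestPawn's UserPrincessNow flag changes.
; Tick drives movement, pauses on Block hits, and teleports it to ChangePrincess's spot or parks it high up on a swap, using Delays.
; Capsule hits check tags across the hit actor's class to set block, death and goal flags.
; BP_BackBoss proximity also kills, death disables collision, and clearing fades the camera.
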(event `self.ReceiveBeginPlay`
  ;[1 1 1] 初期化
  (set `self.BlockHit` false)
  (set `self.NeedleHit` false)
  (set `self.DevilHit` false)
  (set `self.Location` (`self.K2_GetActorLocation`))
  (set `self.Rotation` (`self.K2_GetActorRotation`))
  (set `self.DeathNow` false)
  (`PrimitiveComponent.SetCollisionEnabled` (`self.CapsuleComponent`) "QueryAndPhysics")
  (`PrimitiveComponent.SetCollisionEnabled` (`self.Mesh`) "QueryAndPhysics"))

(event `self.ReceiveTick`
  (params (DeltaSeconds :type "Float (single-precision)"))
  (bind (_returnvalue_x _returnvalue_y) (`KismetMathLibrary.BreakVector` (`self.GetActorForwardVector`)))
  (bind (_returnvalue_x_2 _returnvalue_y_2 _returnvalue_z) (`KismetMathLibrary.BreakVector` (`self.K2_GetActorLocation`)))
  (bind (_location_x _location_y) (`KismetMathLibrary.BreakVector` (`self.Location`)))
  (bind (_location_x_2 _location_y_2) (`KismetMathLibrary.BreakVector` (`self.Location`)))
  (bind _location_x_3 (`KismetMathLibrary.BreakVector` (`self.Location`)))
  (bind (_location_x_4 _location_y_3) (`KismetMathLibrary.BreakVector` (`/Game/My/BP/BP_ChangePrincess.Location` (`self.ChangePrincess`))))
  (if (`self.UserPrincessNow`)
    (bind _outactors (`GameplayStatics.GetAllActorsOfClass` "/Game/My/BP/BP_BackBoss.BP_BackBoss_C"))
    (for _array_element _outactors
      (bind (_location_x_5 _location_y_4) (`KismetMathLibrary.BreakVector` (`/Game/My/BP/BP_BackBoss.location` _array_element)))
      (if (`KismetMathLibrary.NearlyEqual_FloatFloat` _location_y_4 _location_y_2 100.0)
        (set `self.DeathNow` true)
        ;[1 1 1] 死んだら
        (`PrimitiveComponent.SetCollisionEnabled` (`self.Mesh`) "NoCollision" :!label _label)
        (`PrimitiveComponent.SetCollisionEnabled` (`self.CapsuleComponent`) "NoCollision")
        (else
          (if (`self.Clear`) :!label _label_2
            (`PlayerCameraManager.StartCameraFade` (`GameplayStatics.GetPlayerCameraManager` 0) 0.1 1.0 4.0 (struct :`R` 0.963013 :`G` 1.0 :`B` 0.431647 :`A` 1.0) false true)
            (else
              ;[1 1 1] 当たってるかどうか
              (if (`self.BlockHit`)
                (`KismetSystemLibrary.Delay` 0.5)
                (set `self.BlockHit` false)
                ;[1 1 1] ユーザーの使うキャラと相違があるか判定
                (bind _asbp_test_pawn (cast `/Game/My/BP/BP_TestPawn` (`GameplayStatics.GetPlayerPawn` 0) :!label _label_3))
                (bind _userprincessnow (`/Game/My/BP/BP_TestPawn.UserPrincessNow` _asbp_test_pawn))
                (if (!= (`self.UserPrincessNow`) _userprincessnow)
                  (set `self.ChangeNow` true)
                  (bind _output_get (set `self.UserPrincessNow` _userprincessnow))
                  (`KismetSystemLibrary.Delay` 1.5)
                  (set `self.BlockHit` false)
                  (if _output_get
                    ;[1 1 1] 自分になるとき
                    (`self.K2_SetActorLocation` (`KismetMathLibrary.MakeVector` _location_x_4 (- _location_y_3 -45.0) 160.0) false true)
                    (`self.K2_SetActorRotation` (`/Game/My/BP/BP_ChangePrincess.Rotation` (`self.ChangePrincess`)))
                    (else
                      ;[1 1 1] 自分じゃなくなる時
                      (`self.K2_SetActorLocation` (`KismetMathLibrary.MakeVector` _location_x _location_y 2600.0) false true)
                      (`self.K2_SetActorRotation` (`self.Rotation`)))))
                (elif (`self.NeedleHit`)
                  _
                  (elif (not (`self.DevilHit`))
                    ;[1 1 1] 死んでいない
                    (if (`self.DeathNow`)
                      (goto _label)
                      (else
                        (if (`self.ChangeNow`)
                          (`KismetSystemLibrary.Delay` 3.0)
                          (set `self.ChangeNow` false))
                        ;[1 1 1] 当たっていなかったら移動し続ける
                        (`self.AddMovementInput` (`KismetMathLibrary.MakeVector` 0.0 _returnvalue_y))
                        (set `self.Location` (`KismetMathLibrary.MakeVector` _location_x_3 _returnvalue_y_2 _returnvalue_z))
                        (`self.K2_SetActorRotation` (`self.Rotation`))
                        (goto _label_3)))))))))))
    (else
      (goto _label_2))))

(event `self.CapsuleComponent.OnComponentHit`
  (params (HitComponent :type "PrimitiveComponent Object Reference") (OtherActor :type "Actor Object Reference") (OtherComp :type "PrimitiveComponent Object Reference") (NormalImpulse :type "Vector Structure") (Hit :type "HitResult Structure (by ref)"))
  ;[1 1 1] 当たったら
  (`self.MyComponentBlockHit` OtherActor)
  (`self.MyComponentNeedleHit` OtherActor)
  (`self.MyComponentDevilHit` OtherActor)
  (`self.MyComponentGoalHit` OtherActor)
  (`self.MyComponentGolemHit` OtherActor))

(fn `MyComponentBlockHit`
  (params (OtherActor :type "Actor Object Reference"))
  (bind _outactors (`GameplayStatics.GetAllActorsOfClass` (`GameplayStatics.GetObjectClass` OtherActor)))
  (for _array_element _outactors
    (set `self.BlockHit` (`self.ActorHasTag` _array_element "Block"))))

(fn `MyComponentDevilHit`
  (params (`Other Actor` :type "Actor Object Reference"))
  (bind _outactors (`GameplayStatics.GetAllActorsOfClass` (`GameplayStatics.GetObjectClass` `Other Actor`)))
  (for _array_element _outactors
    (bind _output_get (set `self.DevilHit` (`self.ActorHasTag` _array_element "Devil")))
    (if _output_get
      (`/Engine/EditorBlueprintResources/StandardMacros.DoOnce` false
        (:`Completed`
          (set `self.DeathNow` true))))))

(fn `MyComponentGoalHit`
  (params (`Other Actor` :type "Actor Object Reference"))
  (bind _outactors (`GameplayStatics.GetAllActorsOfClass` (`GameplayStatics.GetObjectClass` `Other Actor`)))
  (for _array_element _outactors
    (if (`self.ActorHasTag` _array_element "Goal")
      (set `self.Clear` true))))

(fn `MyComponentGolemHit`
  (params (`Other Actor` :type "Actor Object Reference"))
  (bind _outactors (`GameplayStatics.GetAllActorsOfClass` (`GameplayStatics.GetObjectClass` `Other Actor`)))
  (for _array_element _outactors
    (set `self.DeathNow` (`self.ActorHasTag` _array_element "Golem"))))

(fn `MyComponentNeedleHit`
  (params (OtherActor :type "Actor Object Reference"))
  (bind _outactors (`GameplayStatics.GetAllActorsOfClass` (`GameplayStatics.GetObjectClass` OtherActor)))
  (for _array_element _outactors
    (bind _output_get (set `self.NeedleHit` (`self.ActorHasTag` _array_element "Needle")))
    (if _output_get
      (`/Engine/EditorBlueprintResources/StandardMacros.DoOnce` false
        (:`Completed`
          (set `self.DeathNow` true))))))

(fn `UserConstructionScript`)