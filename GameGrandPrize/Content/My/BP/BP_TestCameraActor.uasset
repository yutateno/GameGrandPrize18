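; Test camera actor that follows the active princess character along the Y axis, keeping the X and Z captured from its camera component at BeginPlay.
; Every Tick it finds the normal and transformed princesses by actor tag and caches their positions.
; BP_TestPawn's UserPrincessNow flag selects which Y to copy, and the camera component moves there with sweep and teleport enabled.
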(event `self.ReceiveBeginPlay`
  (bind (_princesslocation_x _princesslocation_y) (`KismetMathLibrary.BreakVector` (`self.PrincessLocation`)))
  (bind (_location_x _location_y _location_z) (`KismetMathLibrary.BreakVector` (`self.location`)))
  (set `self.location` (`SceneComponent.K2_GetComponentLocation` (`self.CameraComponent`)))
  (bind _outactors (`GameplayStatics.GetAllActorsWithTag` "MainCharacter_P"))
  (for _array_element _outactors
    (set `self.PrincessLocation` (`self.K2_GetActorLocation` _array_element))
    (bind _outactors_2 (`GameplayStatics.GetAllActorsWithTag` "MainCharacter_CP"))
    (for _array_element_2 _outactors_2
      (set `self.ChangePrincessLocation` (`self.K2_GetActorLocation` _array_element_2))
      (set `self.location` (`KismetMathLibrary.MakeVector` _location_x _princesslocation_y _location_z)))))

(event `self.ReceiveTick`
  (params (DeltaSeconds :type "Float (single-precision)"))
  (bind (_location_x _location_y _location_z) (`KismetMathLibrary.BreakVector` (`self.location`)))
  (bind (_changeprincesslocation_x _changeprincesslocation_y) (`KismetMathLibrary.BreakVector` (`self.ChangePrincessLocation`)))
  (bind (_princesslocation_x _princesslocation_y) (`KismetMathLibrary.BreakVector` (`self.PrincessLocation`)))
  (bind (_location_x_2 _location_y_2 _location_z_2) (`KismetMathLibrary.BreakVector` (`self.location`)))
  (bind _outactors (`GameplayStatics.GetAllActorsWithTag` "MainCharacter_P"))
  (for _array_element _outactors
    (set `self.PrincessLocation` (`self.K2_GetActorLocation` _array_element))
    (bind _outactors_2 (`GameplayStatics.GetAllActorsWithTag` "MainCharacter_CP"))
    (for _array_element_2 _outactors_2
      (set `self.ChangePrincessLocation` (`self.K2_GetActorLocation` _array_element_2))
      (bind _asbp_test_pawn (cast `/Game/My/BP/BP_TestPawn` (`GameplayStatics.GetPlayerPawn` 0)))
      (if (`/Game/My/BP/BP_TestPawn.UserPrincessNow` _asbp_test_pawn)
        ;[1 1 1] 通常姫時
        (bind _output_get (set `self.location` (`KismetMathLibrary.MakeVector` _location_x_2 _princesslocation_y _location_z_2)))
        (`SceneComponent.K2_SetWorldLocation` (`self.CameraComponent`) _output_get true true)
        (else
          ;[1 1 1] 変身姫時
          (bind _output_get_2 (set `self.location` (`KismetMathLibrary.MakeVector` _location_x _changeprincesslocation_y _location_z)))
          (`SceneComponent.K2_SetWorldLocation` (`self.CameraComponent`) _output_get_2 true true))))))

(fn `UserConstructionScript`)