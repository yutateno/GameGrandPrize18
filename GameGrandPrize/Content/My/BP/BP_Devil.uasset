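; BP_Devil is a character that walks along its forward Y direction once the player pawn's AnyButtonCheck is set.
; Capsule hits set flags by checking tags on all actors of the hit actor's class.
; Tick reads them: princess and block hits delay movement; needles, changed-princess hits (delayed) or nearing a BP_BackBoss on Y cause death.
; Death disables mesh and capsule collision, then destroys the actor after a short delay.
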(event `self.ReceiveBeginPlay`
  ;[1 1 1] 初期化
  (set `self.PrincessHit` false)
  (set `self.DeathNow` false)
  (set `self.BlockHit` false)
  (set `self.ChangPrincessHit` false))

(event `self.ReceiveTick`
  (params (DeltaSeconds :type "Float (single-precision)"))
  (bind (_returnvalue_x _returnvalue_y) (`KismetMathLibrary.BreakVector` (`self.GetActorForwardVector`)))
  (bind (_returnvalue_x_2 _returnvalue_y_2) (`KismetMathLibrary.BreakVector` (`self.K2_GetActorLocation`)))
  (bind _asbp_test_pawn (cast `/Game/My/BP/BP_TestPawn` (`GameplayStatics.GetPlayerPawn` 0)))
  (if (`/Game/My/BP/BP_TestPawn.AnyButtonCheck` _asbp_test_pawn)
    (bind _outactors (`GameplayStatics.GetAllActorsOfClass` "/Game/My/BP/BP_BackBoss.BP_BackBoss_C"))
    (for _array_element _outactors
      (bind (_location_x _location_y) (`KismetMathLibrary.BreakVector` (`/Game/My/BP/BP_BackBoss.location` _array_element)))
      (if (== (`KismetMathLibrary.MakeVector` 0.0 _location_y) (`KismetMathLibrary.MakeVector` 0.0 _returnvalue_y_2) :`ErrorTolerance` 300.0)
        (set `self.DeathNow` true)
        ;[1 1 1] 死んだら
        (`PrimitiveComponent.SetCollisionEnabled` (`self.Mesh`) "NoCollision" :!label _label)
        (`PrimitiveComponent.SetCollisionEnabled` (`self.CapsuleComponent`) "NoCollision")
        (`KismetSystemLibrary.Delay` 0.7)
        (`self.K2_DestroyActor`)
        (else
          ;[1 1 1] どこにもあたっていなかったら動き続ける
          (if (`self.PrincessHit`)
            (`KismetSystemLibrary.Delay` 1.0)
            (set `self.PrincessHit` false))
          (if (`self.DeathNow`)
            (goto _label)
            (else
              (if (`self.BlockHit`)
                ;[1 1 1] ブロックに当たったら破壊モーション中delayかけてから解除
                (`KismetSystemLibrary.Delay` 0.5)
                (set `self.BlockHit` false))
              (if (`self.ChangPrincessHit`)
                ;[1 1 1] やべぇ姫にぶち当たったら
                (`KismetSystemLibrary.Delay` 2.64)
                (`/Engine/EditorBlueprintResources/StandardMacros.DoOnce` false
                  (:`Completed`
                    (set `self.DeathNow` true)
                    (goto _label)))
                (else
                  (`self.AddMovementInput` (`KismetMathLibrary.MakeVector` 0.0 _returnvalue_y)))))))))))

(event `self.CapsuleComponent.OnComponentHit`
  (params (HitComponent :type "PrimitiveComponent Object Reference") (OtherActor :type "Actor Object Reference") (OtherComp :type "PrimitiveComponent Object Reference") (NormalImpulse :type "Vector Structure") (Hit :type "HitResult Structure (by ref)"))
  ;[1 1 1] 当たったら
  (`self.MyFunc_ChangePrincessHit` OtherActor)
  (`self.MyFunc_PrincessHit` OtherActor)
  (`self.MyFunc_BlockHit` OtherActor)
  (`self.MyFunc_NeedleHit` OtherActor))

(fn `MyFunc_BlockHit`
  (params (`Other Actor` :type "Actor Object Reference"))
  (bind _outactors (`GameplayStatics.GetAllActorsOfClass` (`GameplayStatics.GetObjectClass` `Other Actor`)))
  (for _array_element _outactors
    (set `self.BlockHit` (`self.ActorHasTag` _array_element "Block"))))

(fn `MyFunc_ChangePrincessHit`
  (params (`Other Actor` :type "Actor Object Reference"))
  (bind _outactors (`GameplayStatics.GetAllActorsOfClass` (`GameplayStatics.GetObjectClass` `Other Actor`)))
  (for _array_element _outactors
    (set `self.ChangPrincessHit` (`self.ActorHasTag` _array_element "MainCharacter_CP"))))

(fn `MyFunc_NeedleHit`
  (params (`Other Actor` :type "Actor Object Reference"))
  (bind _outactors (`GameplayStatics.GetAllActorsOfClass` (`GameplayStatics.GetObjectClass` `Other Actor`)))
  (for _array_element _outactors
    (if (`self.ActorHasTag` _array_element "Needle")
      (`/Engine/EditorBlueprintResources/StandardMacros.DoOnce` false
        (:`Completed`
          (set `self.DeathNow` true))))))

(fn `MyFunc_PrincessHit`
  (params (`Other Actor` :type "Actor Object Reference"))
  (bind _outactors (`GameplayStatics.GetAllActorsOfClass` (`GameplayStatics.GetObjectClass` `Other Actor`)))
  (for _array_element _outactors
    (if (`self.ActorHasTag` _array_element "MainCharacter_P")
      (`/Engine/EditorBlueprintResources/StandardMacros.DoOnce` false
        (:`Completed`
          (set `self.PrincessHit` true))))))

(fn `UserConstructionScript`)