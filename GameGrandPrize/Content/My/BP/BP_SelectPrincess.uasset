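; BP_SelectPrincess is the stage-select character that walks between two end points to choose the Tutorial or Main level.
; Left and Right inputs set flags that Tick uses to step Y between fixed limits, turning mesh and spring arm, with delayed footstep sounds.
; Select at either end shows a loading widget and opens that level.
; Back pauses the game and shows a quit prompt, swapping two widgets for left (quit) and right (resume).
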(event `self.ReceiveBeginPlay`
  (bind (_returnvalue_x _returnvalue_y _returnvalue_z) (`KismetMathLibrary.BreakVector` (`self.K2_GetActorLocation`)))
  (set `self.Y` _returnvalue_y)
  (set `self.X` _returnvalue_x)
  (set `self.Z` _returnvalue_z)
  (bind _returnvalue (`|CreateWidget` "/Game/My/UI/UMG_EndLeft.UMG_EndLeft_C"))
  (set `self.UMG_End_Left` _returnvalue)
  (bind _returnvalue_2 (`|CreateWidget` "/Game/My/UI/UMG_EndRight.UMG_EndRight_C"))
  (set `self.UMG_End_Right` _returnvalue_2))

(event `InputAction|ActionLeft`
  (params (Key :type "Key Structure"))
  (:`Pressed`
    (if (not (<= (`self.Y`) 0.0))
      (set `self.leftflag` true))))

(event `InputAction|ActionRight`
  (params (Key :type "Key Structure"))
  (:`Pressed`
    (if (not (>= (`self.Y`) 520.0))
      (set `self.rightflag` true))))

(event `self.ReceiveTick`
  (params (DeltaSeconds :type "Float (single-precision)"))
  (if (`self.rightflag`)
    (if (>= (`self.Y`) 520.0)
      (set `self.rightflag` false)
      (else
        (bind _output_get (set `self.Y` (+ (`self.Y`) 5.0)))
        (`self.K2_SetActorLocation` (`KismetMathLibrary.MakeVector` (`self.X`) _output_get (`self.Z`)))
        (`SceneComponent.K2_SetRelativeRotation` (`self.Mesh`) (struct :`Yaw` -90.0) false false)
        (`SceneComponent.K2_SetRelativeRotation` (`self.SpringArm`) (struct :`Pitch` -30.0) false false)
        (`KismetSystemLibrary.Delay` 0.4)
        (`GameplayStatics.PlaySoundAtLocation` "/Game/My/Sound/Cue/C_Foot.C_Foot" (`self.K2_GetActorLocation`))))
    (elif (`self.leftflag`)
      (if (<= (`self.Y`) 0.0)
        (set `self.leftflag` false)
        (else
          (bind _output_get_2 (set `self.Y` (+ (`self.Y`) -5.0)))
          (`self.K2_SetActorLocation` (`KismetMathLibrary.MakeVector` (`self.X`) _output_get_2 (`self.Z`)))
          (`SceneComponent.K2_SetRelativeRotation` (`self.Mesh`) (struct :`Yaw` 90.0) false false)
          (`SceneComponent.K2_SetRelativeRotation` (`self.SpringArm`) (struct :`Pitch` -30.0 :`Yaw` -180.0) false false)
          (`KismetSystemLibrary.Delay` 0.4)
          (`GameplayStatics.PlaySoundAtLocation` "/Game/My/Sound/Cue/C_Foot.C_Foot" (`self.K2_GetActorLocation`)))))))

(event `InputAction|ActionSelect`
  (params (Key :type "Key Structure"))
  (bind _y (`self.Y`))
  (:`Pressed`
    (`GameplayStatics.PlaySound2D` "/Game/My/Sound/Cue/C_StageSelect.C_StageSelect")
    (if (== _y 0.0)
      (bind _returnvalue (`|CreateWidget` "/Game/My/UI/UMG_Loading.UMG_Loading_C"))
      (`UserWidget.AddToViewport` _returnvalue 0)
      (`KismetSystemLibrary.Delay` 2.0)
      (`WidgetBlueprintLibrary.SetInputMode_GameAndUIEx` (`GameplayStatics.GetPlayerController` 0))
      (`GameplayStatics.OpenLevel` "Tutorial")
      (elif (== _y 520.0)
        (bind _returnvalue_2 (`|CreateWidget` "/Game/My/UI/UMG_Loading.UMG_Loading_C"))
        (`UserWidget.AddToViewport` _returnvalue_2 0)
        (`KismetSystemLibrary.Delay` 2.0)
        (`WidgetBlueprintLibrary.SetInputMode_GameAndUIEx` (`GameplayStatics.GetPlayerController` 0))
        (`GameplayStatics.OpenLevel` "Main")))))

(event `InputAction|ActionEndBack`
  (params (Key :type "Key Structure"))
  (:`Pressed`
    (set `self.EndOptionNow` true)
    (`UserWidget.AddToViewport` (`self.UMG_End_Right`) 0)
    (set `self.umgLeftFLag` false)
    (`GameplayStatics.SetGamePaused` true)))

(event `InputAction|ActionEndNow_A` :paused true
  (params (Key :type "Key Structure"))
  (:`Pressed`
    (if (`self.EndOptionNow`)
      (set `self.EndOptionNow` false)
      (if (`self.EndOptionLeft`)
        (`GameplayStatics.SetGamePaused` false)
        (`GameplayStatics.PlaySound2D` "/Game/My/Sound/Cue/C_End.C_End")
        (`KismetSystemLibrary.QuitGame` null "Quit")
        (else
          (`Widget.RemoveFromParent` (`self.UMG_End_Right`))
          (`GameplayStatics.SetGamePaused` false)
          (`GameplayStatics.PlaySound2D` "/Game/My/Sound/Cue/C_EndBack.C_EndBack"))))))

(event `InputAction|ActionEndNow_Left` :paused true
  (params (Key :type "Key Structure"))
  (:`Pressed`
    (if (`self.EndOptionNow`)
      (set `self.EndOptionLeft` true)
      (if (not (`self.umgLeftFLag`))
        (`Widget.RemoveFromParent` (`self.UMG_End_Right`))
        (`UserWidget.AddToViewport` (`self.UMG_End_Left`) 0)
        (set `self.umgLeftFLag` true)))))

(event `InputAction|ActionEndNow_Right` :paused true
  (params (Key :type "Key Structure"))
  (:`Pressed`
    (if (`self.EndOptionNow`)
      (set `self.EndOptionLeft` false)
      (if (`self.umgLeftFLag`)
        (`Widget.RemoveFromParent` (`self.UMG_End_Left`))
        (`UserWidget.AddToViewport` (`self.UMG_End_Right`) 0)
        (set `self.umgLeftFLag` false)))))

(fn `UserConstructionScript`)