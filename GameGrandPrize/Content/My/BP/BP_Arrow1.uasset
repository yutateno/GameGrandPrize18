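; BP_Arrow1 is an arrow actor that spawns a circle particle effect when its ClickCheck flag turns on.
; It caches its location at BeginPlay, and Tick stores its rotation and polls ClickCheck, which is set outside these graphs.
; Two latch flags limit spawning to one scaled-up MP_Circle per activation, attached to Ypaneru at the cached world location.
; Turning ClickCheck off only re-arms the latch, leaving the stored emitter untouched.
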(event `self.ReceiveBeginPlay`
  (set `self.Location` (`self.K2_GetActorLocation`)))

(event `self.ReceiveTick`
  (params (DeltaSeconds :type "Float (single-precision)"))
  (set `self.rotatiron` (`self.K2_GetActorRotation`))
  (if (`self.ClickCheck`)
    (if (not (`self.EmitterFlag`))
      (set `self.EmitterFlag` true)
      (bind _returnvalue (`GameplayStatics.SpawnEmitterAttached` "/Game/My/Effect/MP_Circle.MP_Circle" (`self.y-paneru`) "None" (`self.Location`) (struct) (5.0 5.0 5.0) "KeepWorldPosition"))
      (set `self.AfterEmitterFlag` false)
      (set `self.PaneruEmitter` _returnvalue))
    (elif (not (`self.AfterEmitterFlag`))
      (set `self.AfterEmitterFlag` true)
      (set `self.EmitterFlag` false))))

(fn `UserConstructionScript`)