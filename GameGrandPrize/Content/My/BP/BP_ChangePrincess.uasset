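; BP_ChangePrincess is the swappable princess character, which moves itself along its forward Y axis each tick.
; Capsule hits set Block, Needle or Devil flags from tags on the hit actor's class instances, pausing movement until Tick-driven Delays clear them.
; When BP_TestPawn's UserPrincessNow flag changes, it waits, then teleports either out of play high above or beside the Princess reference to take over.
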(event `self.ReceiveBeginPlay`
  ;[1 1 1] 初期化
  (set `self.BlockHit` false)
  (set `self.NeedleHit` false)
  (set `self.DevilHit` false)
  (set `self.Location` (`self.K2_GetActorLocation`))
  (set `self.Rotation` (`self.K2_GetActorRotation`)))

(event `self.ReceiveTick`
  (params (DeltaSeconds :type "Float (single-precision)"))
  (bind (_returnvalue_x _returnvalue_y) (`KismetMathLibrary.BreakVector` (`self.GetActorForwardVector`)))
  (bind (_returnvalue_x_2 _returnvalue_y_2 _returnvalue_z) (`KismetMathLibrary.BreakVector` (`self.K2_GetActorLocation`)))
  (bind (_location_x _location_y) (`KismetMathLibrary.BreakVector` (`self.Location`)))
  (bind _location_x_2 (`KismetMathLibrary.BreakVector` (`self.Location`)))
  (bind (_location_x_3 _location_y_2) (`KismetMathLibrary.BreakVector` (`/Game/My/BP/BP_Princess.Location` (`self.Princess`))))
  (if (`self.BlockHit`)
    (`KismetSystemLibrary.Delay` 0.5 :!label _label)
    (set `self.BlockHit` false)
    (`KismetSystemLibrary.Delay` 0.5)
    (set `self.NeedleHit` false)
    (elif (`self.NeedleHit`)
      (goto _label)
      (elif (`self.DevilHit`)
        (`KismetSystemLibrary.Delay` 2.64)
        (set `self.DevilHit` false)
        (else
          (if (`self.ChangeNow`)
            (`KismetSystemLibrary.Delay` 3.0)
            (set `self.ChangeNow` false))
          ;[1 1 1] 動き
          (`self.AddMovementInput` (`KismetMathLibrary.MakeVector` 0.0 _returnvalue_y))
          (set `self.Location` (`KismetMathLibrary.MakeVector` _location_x_2 _returnvalue_y_2 _returnvalue_z))
          (`self.K2_SetActorRotation` (`self.Rotation`))
          ;[1 1 1] ユーザーが使うキャラについて
          (bind _asbp_test_pawn (cast `/Game/My/BP/BP_TestPawn` (`GameplayStatics.GetPlayerPawn` 0)))
          (bind _userprincessnow (`/Game/My/BP/BP_TestPawn.UserPrincessNow` _asbp_test_pawn))
          ;;[1 0.9101 0.5277] ユーザーが使うキャラについて現状と違うか判定
          (if (!= (`self.UserPrincessNow`) _userprincessnow)
            (set `self.ChangeNow` true)
            (bind _output_get (set `self.UserPrincessNow` _userprincessnow))
            (`KismetSystemLibrary.Delay` 1.5)
            (if _output_get
              ;[1 1 1] 自分じゃなくなるとき
              (`self.K2_SetActorLocation` (`KismetMathLibrary.MakeVector` _location_x _location_y 2600.0) false true)
              (`self.K2_SetActorRotation` (`self.Rotation`))
              (else
                ;[1 1 1] 自分になるとき
                (`self.K2_SetActorLocation` (`KismetMathLibrary.MakeVector` _location_x_3 (- _location_y_2 -45.0) 160.0) false true)
                (`self.K2_SetActorRotation` (`/Game/My/BP/BP_Princess.Rotation` (`self.Princess`)))))))))))

(event `self.CapsuleComponent.OnComponentHit`
  (params (HitComponent :type "PrimitiveComponent Object Reference") (OtherActor :type "Actor Object Reference") (OtherComp :type "PrimitiveComponent Object Reference") (NormalImpulse :type "Vector Structure") (Hit :type "HitResult Structure (by ref)"))
  ;[1 1 1] 当たったら
  (`self.MyBlockHit` OtherActor)
  (`self.MyNeedleHit` OtherActor)
  (`self.MyDevilHit` OtherActor))

(fn `MyBlockHit`
  (params (OtherActor :type "Actor Object Reference"))
  (bind _outactors (`GameplayStatics.GetAllActorsOfClass` (`GameplayStatics.GetObjectClass` OtherActor)))
  (for _array_element _outactors
    (set `self.BlockHit` (`self.ActorHasTag` _array_element "Block"))))

(fn `MyDevilHit`
  (params (`Other Actor` :type "Actor Object Reference"))
  (bind _outactors (`GameplayStatics.GetAllActorsOfClass` (`GameplayStatics.GetObjectClass` `Other Actor`)))
  (for _array_element _outactors
    (set `self.DevilHit` (`self.ActorHasTag` _array_element "Devil"))))

(fn `MyNeedleHit`
  (params (OtherActor :type "Actor Object Reference"))
  (bind _outactors (`GameplayStatics.GetAllActorsOfClass` (`GameplayStatics.GetObjectClass` OtherActor)))
  (for _array_element _outactors
    (set `self.NeedleHit` (`self.ActorHasTag` _array_element "Needle"))))

(fn `UserConstructionScript`)